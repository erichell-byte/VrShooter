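; Login menu pawn that presents the main menu in VR on Oculus Quest or as a screen widget otherwise.
; BeginPlay checks the device, enabling ticking on the 3D menu widget for Quest, or creating a viewport menu with a mouse cursor.
; Left and right widget interaction inputs simulate left mouse clicks on the 3D widgets.
; ToggleServerWidget swaps visibility between the main menu and server widgets.
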(event EventBeginPlay
  (bind _main_menu_widget (Variables|Default|GetMain%20Menu%20Widget))
  (bind _oculus_quest (CallFunction|IsOculusQuestDevice))
  (if _oculus_quest ; Use 3d widget instead of screen widget \nif player is using an Oculus Quest
    ;[0.494 0.3303 1] Show/hide 3d menu
    (Class|WidgetComponent|SetTickMode _main_menu_widget "Enabled")
    (else
      (Class|WidgetComponent|SetTickMode _main_menu_widget "Disabled")
      ;[0.494 0.3303 1] Create login widget
      (Development|PrintString "Log in pawn spawned" true true "(R=0.105407,G=1.000000,B=0.000000,A=1.000000)" 6.0)
      (bind _returnvalue (UserInterface|CreateWidget "/Game/VR_Weapons/Networking/Widgets/Login/Widget_MainMenu.Widget_MainMenu_C" (Game|GetPlayerController 0)))
      (bind _output_get (Variables|Default|SetMain%20menu _returnvalue))
      (UserInterface|Viewport|AddtoViewport _output_get 0)
      (Variables|/Script/Engine.PlayerController|SetbShowMouseCursor (Game|GetPlayerController 0) true))))

(event Input|ActionEvents|InputActionWidgetinteractionright
  (params (Key :type Key%20Structure :default "None"))
  (bind _rightwidgetinteraction (Variables|Default|GetRightWidgetInteraction))
  ;[0 0 0] Widget interaction
  (:Pressed
    (Class|WidgetInteractionComponent|PressPointerKey _rightwidgetinteraction "LeftMouseButton"))
  (:Released
    (Class|WidgetInteractionComponent|ReleasePointerKey _rightwidgetinteraction "LeftMouseButton")))

(event Input|ActionEvents|InputActionWidgetinteractionleft
  (params (Key :type Key%20Structure :default "None"))
  (bind _leftwidgetinteraction (Variables|Default|GetLeftWidgetInteraction))
  ;[0 0 0] Widget interaction
  (:Pressed
    (Class|WidgetInteractionComponent|PressPointerKey _leftwidgetinteraction "LeftMouseButton"))
  (:Released
    (Class|WidgetInteractionComponent|ReleasePointerKey _leftwidgetinteraction "LeftMouseButton")))

(fn ConstructionScript)

(fn ToggleServerWidget
  (params (bNewVisibility :type Boolean))
  (bind _main_menu_widget (Variables|Default|GetMain%20Menu%20Widget))
  (bind _server_widget (Variables|Default|GetServer%20Widget))
  (if bNewVisibility
    (Rendering|SetVisibility _main_menu_widget false false)
    (Rendering|SetVisibility _server_widget true false)
    (else
      (Rendering|SetVisibility _main_menu_widget true false)
      (Rendering|SetVisibility _server_widget false false))))