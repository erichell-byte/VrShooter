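; BP_Assault_rifle is a VR assault rifle that adds a bolt catch/release paddle to its parent weapon.
; Firing with an empty or missing magazine flags the bolt as retracted.
; The owner's free motion controller can touch the paddle, triggering haptics and a server update that chambers a round from the magazine, with a replicated release sound.
; Construction attaches the ejector mesh to the charging handle and applies the sights mesh.
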(event OnComponentBeginOverlap(Boltcatch/releasepaddlecollision)
  (params (OverlappedComponent :type Primitive%20Component%20Object%20Reference) (OtherActor :type Actor%20Object%20Reference) (OtherComp :type Primitive%20Component%20Object%20Reference) (OtherBodyIndex :type Integer) (bFromSweep :type Boolean) (SweepResult :type Hit%20Result%20Structure%20%28by%20ref%29))
  ;[0 0 0] Bolt catch/release paddle (can be touched as an alternative to the charging handle when loading a new mag)
  (Utilities|IsValid (Variables|Default|GetSecondary%20Motion%20Controller%20BP)
    (:Is%20Not%20Valid
      (bind _asbp_motion_controller (Utilities|Casting|CastToBP_MotionController OtherActor)) ; check overlapping actor is motion controller
      (if (Math|Boolean|ANDBoolean (Variables|Default|GetBolt%20retracted) (not (Variables|Default|GetWeapon%20Cocked)) (== (Components|GetOwner OtherActor) (Components|GetOwner)))
        (Utilities|IsValid (Variables|Default|GetPrimary%20Motion%20Controller%20BP)
          (:Is%20Valid
            (Default|RumbleController _asbp_motion_controller "/Game/VR_Weapons/Pawn/Haptics/Haptics_single.Haptics_single" 0.9 false)
            (Variables|Default|SetBolt%20release true))
          (:Is%20Not%20Valid
            _))
        ;;[0.494 0.3303 1] Update on server
        (CallFunction|ServerUpdateBoltStatusandRounds)))))

(event Custom|Server%20update%20bolt%20status%20and%20rounds
  ;[0 0 0] Bolt catch/release paddle (can be touched as an alternative to the charging handle when loading a new mag)
  ;;[0.494 0.3303 1] Update on server
  (Variables|Default|SetBolt%20release true)
  (Variables|Default|SetBolt%20retracted false)
  (CallFunction|LoadNextRoundIntoChamber) ; Load round from magazine into the chamber
  (if (Variables|Default|GetOne%20in%20the%20chamber) ; If a round was loaded successfully into the chamber then update the magazine to remove that round
    (Default|RemoveRound (Variables|Default|GetMagazine))))

(event Custom|Weapon%20fired_Event
  (bind _magazine (Variables|Default|GetMagazine))
  (Utilities|IsValid _magazine ; magazine in gun
    (:Is%20Valid
      (if (== (Variables|/Game/VR_Weapons/Global/Blueprints/BP_Magazine.BP_Magazine_C|GetRounds _magazine) 0) ; Last round fired
        (Variables|Default|SetBolt%20retracted true :!label _label) ; bolt is ready for quick release paddle
      ))
    (:Is%20Not%20Valid
      (goto _label))))

(event Custom|Set%20sights
  (params (NewMesh :type Static%20Mesh%20Object%20Reference))
  (Components|StaticMesh|SetStaticMesh (Variables|Default|GetSM_sights) NewMesh))

(event EventBeginPlay
  (|CallParentFunction)
  (EventDispatchers|AssignWeaponFired (delegate Custom|Weapon%20fired_Event)))

(fn ConstructionScript
  (|CallParentFunction)
  (Transformation|AttachComponentToComponent (Variables|Default|GetEjector%20mesh) (Variables|Default|GetCharging%20handle%20mesh) "None" "KeepWorld" "KeepWorld" "KeepWorld" true) ; Attach bolt to charging handle so it moves when the charging handle is pulled back/released
  (Components|StaticMesh|SetStaticMesh (Variables|Default|GetSM_sights) (Variables|Default|GetSights%20mesh)))

(fn OnRepBoltRelease
  (if (Variables|Default|GetBolt%20release)
    (Audio|PlaySoundatLocation "/Game/VR_Weapons/Guns/Assault_rifle/Audio/Assault_rifle_charging_handle_release_Cue.Assault_rifle_charging_handle_release_Cue" (Transformation|GetWorldLocation (Variables|Default|GetCharging%20handle%20collision)) "0, 0, 0" 1.0 1.0 0.0 "/Game/VR_Weapons/Global/Audio/Small_object_Attenuation.Small_object_Attenuation" "/Game/VR_Weapons/Global/Audio/WeaponConcurrency.WeaponConcurrency" 0) ; Bolt click
  ))