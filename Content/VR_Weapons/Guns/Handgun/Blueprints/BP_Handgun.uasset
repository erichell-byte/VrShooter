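; VR handgun Blueprint, a child weapon that adds slide and barrel animation to firing.
; Each shot plays a timeline that moves the slide and tilts the barrel; the last shot locks the slide back and emits ejector smoke.
; The locked state goes through server events, clears when the slide is grabbed, and counts as a reset charging handle.
; Tick eases the barrel back to default while the charging handle is engaged.
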(event Custom|Weapon%20fired_Event
  (bind _charging_handle_mesh (Variables|Default|GetCharging%20handle%20mesh))
  (bind _charging_handle_mesh_2 (Variables|Default|GetCharging%20handle%20mesh))
  (bind _returnvalue (Transformation|GetSocketTransform _charging_handle_mesh_2 "Ejector" "RTS_World"))
  (if (not (Variables|Default|GetOne%20in%20the%20chamber))
    (Variables|Default|SetSlide%20retracted true)
    (CallFunction|ServerUpdateSlideState true)
    ;[0 0 0] If last shot is being fired - keep slide fully retracted
    (bind (_direction _slide_position _barrel_tilt) (Timeline|Last%20shot PlayFromStart)
      (:Update
        (Transformation|SetRelativeLocation _charging_handle_mesh (Math|Vector|MakeVector _slide_position 0.0 0.0) false false) ; move slide back
        (Transformation|SetRelativeTransform (Variables|Default|GetSM_handgun_barrel) (Math|Transform|Lerp(Transform) (Variables|Default|GetBarrel%20default) (Variables|Default|GetBarrel%20tilt) _barrel_tilt) false false) ; tilt barrel upwards
      )
      (:Finished
        ;[0 0 0] Spawn smoke
        (CallFunction|ServerSpawnSmokeParticles (.x (Variables|/Script/Engine.SceneComponent|GetRelativeLocation _charging_handle_mesh_2)))
        (Effects|SpawnEmitterAttached "/Game/VR_Weapons/Guns/Handgun/Particles/P_Handgun_ejector_smoke_slide_retracted.P_Handgun_ejector_smoke_slide_retracted" _charging_handle_mesh_2 "Ejector" (.location _returnvalue) (.rotation _returnvalue) "1.000000,1.000000,1.000000" "KeepWorldPosition") ; spawn smoke particle
      ))
    (else
      (bind (_direction_2 _slide_position_2 _barrel_slide) (Timeline|Slide PlayFromStart)
        (:Update
          (Transformation|SetRelativeLocation _charging_handle_mesh (Math|Vector|MakeVector _slide_position_2 0.0 0.0) false false) ; move slide back
          (Transformation|SetRelativeTransform (Variables|Default|GetSM_handgun_barrel) (Math|Transform|Lerp(Transform) (Variables|Default|GetBarrel%20default) (Variables|Default|GetBarrel%20tilt) _barrel_slide) false false) ; tilt barrel
        )))))

(event Custom|Charging%20handle%20grabbed%20event
  (CallFunction|ServerUpdateSlideState false))

(event Custom|Server%20spawn%20smoke%20particles
  (params (New%20Location%20X :type Float%20%28single-precision%29))
  ;[0.494 0.3303 1] Spawn on all clients
  (CallFunction|MulticastSpawnSmokeParticles)
  (Transformation|SetRelativeLocation (Variables|Default|GetCharging%20handle%20mesh) (Math|Vector|MakeVector New%20Location%20X 0.0 0.0) false false) ; move slide back
)

(event Custom|Multicast%20spawn%20smoke%20particles
  (bind _charging_handle_mesh (Variables|Default|GetCharging%20handle%20mesh))
  (bind _returnvalue (Transformation|GetSocketTransform _charging_handle_mesh "Ejector" "RTS_World"))
  ;[0.494 0.3303 1] Spawn on all clients
  ;[0 0 0] Spawn smoke
  (Effects|SpawnEmitterAttached "/Game/VR_Weapons/Guns/Handgun/Particles/P_Handgun_ejector_smoke_slide_retracted.P_Handgun_ejector_smoke_slide_retracted" _charging_handle_mesh "Ejector" (.location _returnvalue) (.rotation _returnvalue) "1.000000,1.000000,1.000000" "KeepWorldPosition") ; spawn smoke particle
)

(event Custom|Server%20update%20slide%20state
  (params (Slide%20retracted :type Boolean))
  ;[0.494 0.3303 1] Update on server
  (Variables|Default|SetSlide%20retracted Slide%20retracted) ; Stops slide being animated back to default position\nin reloading graph
)

(event EventBeginPlay
  (|CallParentFunction)
  (EventDispatchers|AssignWeaponFired (delegate Custom|Weapon%20fired_Event))
  (EventDispatchers|BindEventtoChargingHandleGrabbed (delegate Custom|Charging%20handle%20grabbed%20event)))

(event Collision|EventActorBeginOverlap
  (params (OtherActor :type Actor%20Object%20Reference)))

(event EventTick
  (params (DeltaSeconds :type Float%20%28single-precision%29))
  (|CallParentFunction DeltaSeconds)
  (if (and (!= (Variables|Default|GetPrimary%20Hand%20mesh) 0) (Variables|Default|GetCharging%20Handle%20engaged)) ; if the gun has been cocked but the barrel is not reset then interp barrel back to default position
    (Transformation|SetRelativeTransform (Variables|Default|GetSM_handgun_barrel) (Class|KismetMathLibrary|TInterpto (Transformation|GetRelativeTransform (Variables|Default|GetSM_handgun_barrel)) (Variables|Default|GetBarrel%20default) DeltaSeconds 75.0) false false)))

(fn ConstructionScript
  (|CallParentFunction)
  (Components|DestroyComponent (Variables|Default|GetEjector%20mesh)))

(fn IsChargingHandleReset
  (return (or (|CallParentFunction) (Variables|Default|GetSlide%20retracted))))