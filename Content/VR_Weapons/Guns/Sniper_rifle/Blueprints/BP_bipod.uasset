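; VR sniper rifle bipod that the gun mounts onto and is aimed from via the gripping motion controller.
; Look-at rotation from controller to pivot aims the gun, while distance change slides the rail; leaving the rail range detaches it.
; The controlling client sends transforms and unmounting to the server, Mounted's OnRep reattaches gun to hand, and recoil multicasts.
; Without IK, a gun-attached dummy hand replaces the controller hand while mounted.
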(event Custom|Server%20update%20weapon%20position
  (params (MountedGunRotation :type Rotator) (MountedGunPosition :type Float%20%28single-precision%29))
  ;[0 0 0] Update gun position by rotating the pivot and moving the slider rail
  ; (calculated by measuring Look at Rotation and distance between motion controller and pivot)
  ;;[0.494 0.3303 1] Update mounted weapon transform on server
  (Variables|Default|SetMountedGunRotation MountedGunRotation)
  (Variables|Default|SetMountedGunPosition MountedGunPosition))

(event Custom|Multicast%20animate%20recoil
  ;[0.494 0.3303 1] Replicate recoil on server
  (if (not (Variables|Default|GetLocally%20controlled))
    ;[0 0 0] Recoil
    (bind (_direction _bipod _slider_rail) (Timeline|Bipod%20recoil PlayFromStart)
      (:Update
        (Transformation|SetActorLocation (+ (* (Math|Rotator|GetRotationXVector (Transformation|GetWorldRotation (Variables|Default|GetPivot))) _bipod) (Transformation|GetActorLocation)) false false)
        (Variables|Default|SetSlider%20rail%20offset _slider_rail)))))

(event Custom|Animate%20recoil
  ;[0 0 0] Recoil
  ;;[0.494 0.3303 1] Replicate recoil on server
  (CallFunction|ServerAnimateRecoil)
  (bind (_direction _bipod _slider_rail) (Timeline|Bipod%20recoil PlayFromStart)
    (:Update
      (Transformation|SetActorLocation (+ (* (Math|Rotator|GetRotationXVector (Transformation|GetWorldRotation (Variables|Default|GetPivot))) _bipod) (Transformation|GetActorLocation)) false false)
      (Variables|Default|SetSlider%20rail%20offset _slider_rail))))

(event Custom|Server%20animate%20recoil
  ;[0.494 0.3303 1] Replicate recoil on server
  (CallFunction|MulticastAnimateRecoil))

(event Custom|Set%20is%20locally%20controlled
  (params (Locally%20controlled :type Boolean))
  (bind _output_get (Variables|Default|SetLocally%20controlled Locally%20controlled))
  (if (not _output_get)
    (Variables|Default|SetMotionController 0) ; clear reference when user releases grip
  ))

(event Custom|Server%20remove%20from%20bipod
  ;[0.494 0.3303 1] Update all clients when sniper has been removed
  (Variables|Default|SetMounted false))

(event EventBeginPlay
  ;[1 0.6016 0] Remove dummy mesh
  (Components|DestroyComponent (Variables|Default|GetDummy_mounted_weapon)) ; remove dummy weapon
)

(event EventTick
  (params (DeltaSeconds :type Float%20%28single-precision%29))
  ;[0 0 0] Update gun position by rotating the pivot and moving the slider rail
  ; (calculated by measuring Look at Rotation and distance between motion controller and pivot)
  (Utilities|IsValid (Variables|Default|GetMotionController)
    (:Is%20Valid
      (Utilities|FlowControl|Sequence
        (:then_0
          (if (Variables|Default|GetLocally%20controlled)
            (switch Utilities|FlowControl|Switch|SwitchonE_GripEnum (Variables|/Game/VR_Weapons/Pawn/Blueprints/BP_MotionController.BP_MotionController_C|GetGripState (Variables|Default|GetMotionControllerBP))
              (:NewEnumerator2
                _)
              (:NewEnumerator4
                _))
            (|UpdatePivotrotation) ; Pivot Rotation
            (bind _slider_rail_x_pos (|UpdateSliderrailposition)) ; Slider Location
            (CallFunction|ServerUpdateWeaponPosition (Variables|Default|GetMountedGunRotation) (Variables|Default|GetMountedGunPosition))
            (if (and (or (< _slider_rail_x_pos 0.5) (> _slider_rail_x_pos 24.0)) (Variables|Default|GetMounted))
              (Utilities|Haptics)
              (if (Variables|Default|GetMounted) ; Is this gun still mounted
                ;[0.494 0.3303 1] Update all clients when sniper has been removed
                (Networking|SwitchHasAuthority
                  (:Authority
                    (Variables|Default|SetMounted false))
                  (:Remote
                    (CallFunction|ServerRemovefromBipod)))))))
        (:then_1
          ;;[0 0 0] Update mounted weapon transform
          (Transformation|SetWorldRotation (Variables|Default|GetPivot) (Variables|Default|GetMountedGunRotation) false false)
          (Transformation|SetRelativeLocation (Variables|Default|GetSlider%20Rail%20dummy) (Math|Vector|MakeVector (Variables|Default|GetMountedGunPosition) 0.0 0.0) false false)
          (|Debugging))))))

(fn ConstructionScript)

(fn MountGun
  (bind _debug (Variables|Default|GetDebug))
  (bind _debug_2 (Variables|Default|GetDebug))
  ;[0 0 0] Check gun has not already been mounted
  (if (not (Variables|Default|GetMounted)) ; Don't try to mount weapon if it is already mounted on the bipod
    (Variables|Default|SetMounted true)
    ;[0 0 0] Set slider rail start position
    (Transformation|SetRelativeLocation (Variables|Default|GetSlider%20Rail%20dummy) (Math|Vector|MakeVector (Math|Vector|Distance2D(Vector) (Transformation|GetWorldLocation (Variables|Default|GetSlider%20Rail%20dummy)) (Transformation|GetSocketLocation (Variables|/Game/VR_Weapons/Global/Blueprints/BP_Gun.BP_Gun_C|GetGun%20mesh (Variables|Default|GetBP%20gun)) "Bipod")) 0.0 0.0) false false) ; set slider rail position so its underneath the gun's "bipod" socket
    ;[0 0 0] Attach gun to bipod
    (Transformation|AttachComponentToComponent (Variables|Default|GetBP%20gun) (Variables|Default|GetAttach%20dummy) "" "SnapToTarget" "SnapToTarget" "KeepRelative" true) ; Attach gun to the "Attach dummy". \n\nThis positions the gun correctly on the bipod. \n\nThe Attach dummy is attached to the Slider rail and Pivot \nso the gun can be moved forward/back and rotated in all directions
    (Development|PrintString "Mounted" _debug _debug "(R=0.003254,G=1.000000,B=0.000000,A=1.000000)" 3.0)
    (Transformation|SetActorScale3D (select (Utilities|Enum|Equal(Enum) (Variables|/Game/VR_Weapons/Global/Blueprints/BP_Gun.BP_Gun_C|GetPrimary%20Hand (Variables|Default|GetBP%20gun)) "Left") "1.000000,-1.000000,1.000000" "1.000000,1.000000,1.000000")) ; un-flip sniper if left hand is grabbing
    (|Updatevariablesforhandtracking)
    (Utilities|Haptics)
    (else
      (Development|PrintString "Already mounted" _debug_2 _debug_2 "(R=1.000000,G=0.354956,B=0.000000,A=1.000000)"))))

(fn Show/hideDummyHand
  (params (Hand%20visibility :type Boolean))
  ;[0 0 0] Hides BP motion controller hand mesh. Then shows fake hand attached to rifle. This prevents the real hand mesh from rotating the wrong way and shows the hand mesh as always being aligned to the gun's pistol grip
  (if (and (Utilities|IsValid (Variables|Default|GetMotionControllerBP)) (not (Variables|/Game/VR_Weapons/Global/Blueprints/BP_Gun.BP_Gun_C|GetPawn%20owner%20using%20IK%20body (Variables|Default|GetBP%20gun))))
    (Rendering|SetVisibility (Variables|/Game/VR_Weapons/Pawn/Blueprints/BP_MotionController.BP_MotionController_C|GetHandMesh (Variables|Default|GetMotionControllerBP)) Hand%20visibility false) ; Hide/show real motion controller mesh
    (bind _asbp_sniper_rifle (Utilities|Casting|CastToBP_Sniper_rifle (Variables|Default|GetBP%20gun)))
    (Rendering|SetVisibility (Variables|/Game/VR_Weapons/Guns/Sniper_rifle/Blueprints/BP_Sniper_rifle.BP_Sniper_rifle_C|GetBipod%20dummy%20hand%20right _asbp_sniper_rifle) (not Hand%20visibility) false) ; Hide/show fake motion controller mesh
  ))

(fn GrabGunWhileMounted
  (params (Hand :type EControllerHand%20Enum :default "Left"))
  (bind _debug (Variables|Default|GetDebug))
  (bind _bp_gun (Variables|Default|GetBP%20gun))
  (bind _primary_motion_controller_bp (Variables|/Game/VR_Weapons/Global/Blueprints/BP_Gun.BP_Gun_C|GetPrimary%20Motion%20Controller%20BP _bp_gun))
  (Development|PrintString "Grabbing gun while mounted" _debug _debug "(R=0.000000,G=1.000000,B=0.054240,A=1.000000)" 5.0)
  (Default|InvertChargingHandleGripHand (Variables|Default|GetBP%20gun) false)
  (CallFunction|Show/hideDummyHand false) ; Hide motion controller hand mesh and show fake hand mesh
  (Variables|Default|SetMotionControllerBP _primary_motion_controller_bp) ; Set motion controller actor reference
  (bind _output_get (Variables|Default|SetMotionController (Variables|/Game/VR_Weapons/Pawn/Blueprints/BP_MotionController.BP_MotionController_C|GetMotionController _primary_motion_controller_bp))) ; Set motion controller component  reference
  (Variables|Default|SetStarting%20distance (Math|Vector|Distance(Vector) (Transformation|GetWorldLocation _output_get) (Transformation|GetWorldLocation (Variables|Default|GetSlider%20Rail%20dummy)))) ; Use this as a starting point to measure the motion controller movement
)

(fn OnRepMounted
  (if (not (Variables|Default|GetMounted)) ; Is weapon being mounted?
    (Variables|Default|SetStarting%20distance 0.0)
    (|Attachguntohand)
    (Default|CallGunRemovedfromBipod) ; update sniper
    (CallFunction|Show/hideDummyHand true) ; Show motion controller hand mesh and hide fake hand mesh
  ))