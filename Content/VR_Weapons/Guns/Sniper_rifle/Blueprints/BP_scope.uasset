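; BP_scope is a VR sniper rifle scope that shows a live scene capture on its lens.
; On begin play or player spawn, it feeds a new render target, smaller on Quest, into the capture component and dynamic scope material.
; A 0.25-second loop enables per-frame capture only while the camera is near a recently rendered lens, stopping when the player dies.
; On Quest, the material's vertical tiling is flipped.
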(event Custom|Player%20spawned
  ;[0 0 0] Create new render target
  (bind _oculus_quest (CallFunction|IsOculusQuestDevice))
  (bind _returnvalue (Rendering|CreateRenderTarget2D (Math|Integer|SelectInt 256 512 _oculus_quest) (Math|Integer|SelectInt 256 512 _oculus_quest) "RTF_RGBA16f"))
  ;[0 0 0] Assign render target texture to scene capture camera
  (Rendering|Material|SetTextureParameterValue (Variables|Default|GetScope%20Material) "Render Target Object" _returnvalue)
  (Variables|/Script/Engine.SceneCaptureComponent2D|SetTextureTarget (Variables|Default|GetSceneCaptureComponent2D) _returnvalue)
  (Transformation|SetRelativeScale3D (Variables|Default|GetSceneCaptureComponent2D) "1.000000,1.000000,1.000000")
  (Utilities|FlowControl|Sequence
    (:then_0
      (bind _asmotion_controller_pawn (Utilities|Casting|CastToMotionControllerPawn (Game|Player|GetPlayerPawn 0) :!label _label)
        (:then
          (Variables|Default|SetPlayer _asmotion_controller_pawn)
          (Variables|Default|SetPlayer%20camera (Variables|/Game/VR_Weapons/Pawn/Blueprints/MotionControllerPawn.MotionControllerPawn_C|GetCamera _asmotion_controller_pawn))
          (Rendering|SceneCapture|CaptureScene (Variables|Default|GetSceneCaptureComponent2D) :!class /Script/Engine.SceneCaptureComponent2D)
          (Utilities|FlowControl|Delay 0.25 :!label _label_2)
          (if (not (Variables|/Game/VR_Weapons/Pawn/Blueprints/MotionControllerPawn.MotionControllerPawn_C|GetDead (Variables|Default|GetPlayer)))
            (Variables|/Script/Engine.SceneCaptureComponent|SetbCaptureEveryFrame (Variables|Default|GetSceneCaptureComponent2D) (and (< (Math|Vector|Distance(Vector) (Transformation|GetWorldLocation (Variables|Default|GetPlayer%20camera)) (Transformation|GetWorldLocation (Variables|Default|GetLens))) 75.0) (Class|PrimitiveComponent|WasRecentlyRendered (Variables|Default|GetLens) 0.1)))
            (goto _label_2)))
        (:CastFailed
          (Utilities|FlowControl|Delay 1.0) ; wait for player to spawn
          (goto _label))))
    (:then_1
      (Utilities|FlowControl|Delay 1.0)
      (bind _oculus_quest_2 (CallFunction|IsOculusQuestDevice))
      (if _oculus_quest_2
        (Rendering|Material|SetScalarParameterValue (Variables|Default|GetScope%20Material) "Vtiling" -1.0 :!class /Script/Engine.MaterialInstanceDynamic) ; Flip render target on Oculus Quest
      ))))

(event EventBeginPlay
  ;[0 0 0] Create new render target
  (bind _oculus_quest (CallFunction|IsOculusQuestDevice))
  (bind _returnvalue (Rendering|CreateRenderTarget2D (Math|Integer|SelectInt 256 512 _oculus_quest) (Math|Integer|SelectInt 256 512 _oculus_quest) "RTF_RGBA16f"))
  ;[0 0 0] Assign render target texture to scene capture camera
  (Rendering|Material|SetTextureParameterValue (Variables|Default|GetScope%20Material) "Render Target Object" _returnvalue)
  (Variables|/Script/Engine.SceneCaptureComponent2D|SetTextureTarget (Variables|Default|GetSceneCaptureComponent2D) _returnvalue)
  (Transformation|SetRelativeScale3D (Variables|Default|GetSceneCaptureComponent2D) "1.000000,1.000000,1.000000")
  (Utilities|FlowControl|Sequence
    (:then_0
      (bind _asmotion_controller_pawn (Utilities|Casting|CastToMotionControllerPawn (Game|Player|GetPlayerPawn 0) :!label _label)
        (:then
          (Variables|Default|SetPlayer _asmotion_controller_pawn)
          (Variables|Default|SetPlayer%20camera (Variables|/Game/VR_Weapons/Pawn/Blueprints/MotionControllerPawn.MotionControllerPawn_C|GetCamera _asmotion_controller_pawn))
          (Rendering|SceneCapture|CaptureScene (Variables|Default|GetSceneCaptureComponent2D) :!class /Script/Engine.SceneCaptureComponent2D)
          (Utilities|FlowControl|Delay 0.25 :!label _label_2)
          (if (not (Variables|/Game/VR_Weapons/Pawn/Blueprints/MotionControllerPawn.MotionControllerPawn_C|GetDead (Variables|Default|GetPlayer)))
            (Variables|/Script/Engine.SceneCaptureComponent|SetbCaptureEveryFrame (Variables|Default|GetSceneCaptureComponent2D) (and (< (Math|Vector|Distance(Vector) (Transformation|GetWorldLocation (Variables|Default|GetPlayer%20camera)) (Transformation|GetWorldLocation (Variables|Default|GetLens))) 75.0) (Class|PrimitiveComponent|WasRecentlyRendered (Variables|Default|GetLens) 0.1)))
            (goto _label_2)))
        (:CastFailed
          (Utilities|FlowControl|Delay 1.0) ; wait for player to spawn
          (goto _label))))
    (:then_1
      (Utilities|FlowControl|Delay 1.0)
      (bind _oculus_quest_2 (CallFunction|IsOculusQuestDevice))
      (if _oculus_quest_2
        (Rendering|Material|SetScalarParameterValue (Variables|Default|GetScope%20Material) "Vtiling" -1.0 :!class /Script/Engine.MaterialInstanceDynamic) ; Flip render target on Oculus Quest
      ))))

(event Collision|EventActorBeginOverlap
  (params (OtherActor :type Actor%20Object%20Reference)))

(fn ConstructionScript
  (bind _returnvalue (Rendering|Material|CreateDynamicMaterialInstance (Variables|Default|GetSM_scope) 1 "/Game/VR_Weapons/Guns/Sniper_rifle/Materials/M_scope.M_scope" "None" :!class /Script/Engine.PrimitiveComponent))
  (Variables|Default|SetScope%20Material _returnvalue))