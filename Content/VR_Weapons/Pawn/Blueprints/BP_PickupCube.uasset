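; BP_PickupCube is a networked VR physics cube that motion controllers can pick up and throw, with the weapon-specific interface functions left as stubs.
; Pickup has the pawn request ownership, attaches the cube locally, then polls until the owner is set before calling ServerAttach.
; Drop detaches it, restores physics and passes its velocity to ServerDrop, which replicates the throw through Networking and clears the owner.
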(event Custom|Server%20drop
  (params (Impulse :type Vector))
  (Default|ReplicateActorThrowing (Variables|Default|GetNetworking) (Variables|Debug|GetStaticMeshComponent) Impulse)
  (Actor|SetOwner 0))

(event Custom|Server%20attach
  (params (Hand :type Scene%20Component%20Object%20Reference))
  (Variables|Default|Sethand Hand)
  (Physics|SetSimulatePhysics (Variables|Debug|GetStaticMeshComponent) false)
  (bind _returnvalue (Transformation|AttachComponentToComponent (Variables|Debug|GetStaticMeshComponent) (Variables|Default|Gethand) "PickupCube" "SnapToTarget" "SnapToTarget" "SnapToTarget" false))
  (if _returnvalue
    (Development|PrintString "Cube picked up" true true "(R=0.041247,G=1.000000,B=0.000000,A=1.000000)" 8.0)
    (else
      (Development|PrintString "Cube NOT picked up" true true "(R=1.000000,G=0.000000,B=0.012817,A=1.000000)" 8.0))))

(event Custom|Pickup_Event
  (params (AttachTo :type Scene%20Component%20Object%20Reference) (Hand :type EControllerHand%20Enum :default "Left"))
  (bind _asmotion_controller_pawn (Utilities|Casting|CastToMotionControllerPawn (Game|Player|GetPlayerPawn 0)))
  (Default|ServerSetActorOwnerinPawn _asmotion_controller_pawn self)
  (Physics|SetSimulatePhysics (Variables|Debug|GetStaticMeshComponent) false)
  (Transformation|AttachComponentToComponent (VehicleSound|GetRootComponent) AttachTo "PickupCube" "SnapToTarget" "SnapToTarget" "SnapToTarget" false)
  (if (!= (Components|GetOwner) 0) :!label _label
    (CallFunction|ServerAttach AttachTo)
    (else
      (Utilities|FlowControl|Delay 0.1)
      (goto _label))))

(event EventBeginPlay)

(event Collision|EventActorBeginOverlap
  (params (OtherActor :type Actor%20Object%20Reference)))

(event EventDrop
  (bind _staticmeshcomponent (Variables|Debug|GetStaticMeshComponent))
  (Transformation|DetachFromActor "KeepWorld" "KeepWorld" "KeepWorld")
  (Physics|SetSimulatePhysics _staticmeshcomponent true)
  (CallFunction|ServerDrop (Transformation|GetComponentVelocity _staticmeshcomponent)))

(fn ConstructionScript)

(fn GripHandGuard
  (params (Hand :type BP%20Motion%20Controller%20Object%20Reference))
  (return false 0 "NewEnumerator0"))

(fn InsertMagazine
  (params (OverlappedComponent :type Primitive%20Component%20Object%20Reference) (WeaponType :type E_WeaponType%20Enum :default "NewEnumerator0"))
  (return false 0 0))

(fn Pickup
  (params (Hand :type EControllerHand%20Enum :default "Left") (Grip%20or%20grab :type E_GrabType%20Enum :default "NewEnumerator1") (Motion%20Controller%20Actor :type BP%20Motion%20Controller%20Object%20Reference) (AttachTo :type Scene%20Component%20Object%20Reference))
  (CallFunction|PickupEvent AttachTo Hand)
  (return "NewEnumerator0" false))

(fn PullTrigger
  (return))

(fn ReleaseHandGuard
  (params (Hand :type BP%20Motion%20Controller%20Object%20Reference))
  (return))