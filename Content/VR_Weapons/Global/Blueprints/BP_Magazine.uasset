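; Networked VR weapon magazine that players grab, drop, store in the utility belt, and insert into compatible guns on overlap.
; Pickup and insertion attach locally first to hide latency, then take network ownership and replicate through server events, multicast sounds and a Networking component.
; Construction converts numbered cartridge meshes into instanced meshes to cut draw calls, removed as rounds deplete.
; Empty magazines optionally spawn a replacement when dropped.
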(event OnComponentBeginOverlap(InsertCollision)
  (params (OverlappedComponent :type Primitive%20Component%20Object%20Reference) (OtherActor :type Actor%20Object%20Reference) (OtherComp :type Primitive%20Component%20Object%20Reference) (OtherBodyIndex :type Integer) (bFromSweep :type Boolean) (SweepResult :type Hit%20Result%20Structure%20%28by%20ref%29))
  ;[0 0 0] Insert magazine on overlap
  (Utilities|FlowControl|Delay 0.05)
  (|InsertMagazine OtherActor OtherComp))

(event Custom|Mag%20release%20button
  ;[0.494 0.3303 1] Mag release
  (|Magrelease))

(event Custom|Multicast%20remove%20cartridge%20mesh%20instance
  ;[0.494 0.3303 1] Update cartridge meshes on all clients
  (Class|InstancedStaticMeshComponent|RemoveInstance (Variables|Default|GetISM%20cartridge) (Variables|MagazineSettings|GetRounds)))

(event Custom|Pickup_Event
  (params (Grip%20or%20Grab :type E_GrabType%20Enum :default "NewEnumerator1") (MotionController :type BP%20Motion%20Controller%20Object%20Reference) (Hand :type EControllerHand%20Enum :default "Left") (HandMesh :type Scene%20Component%20Object%20Reference))
  (bind _debug_mode (Variables|MagazineSettings|GetDebug%20mode))
  ;[0 0 0] Pickup/Drop
  (Development|PrintString "Mag pick-up event" _debug_mode _debug_mode)
  (|Pickupmagazine Grip%20or%20Grab MotionController Hand HandMesh))

(event EventBeginPlay
  (Physics|SetSimulatePhysics (Variables|Default|GetMagazine) (Variables|MagazineSettings|GetStart%20simulating%20physics))
  (Variables|/Game/VR_Weapons/Networking/Networking.Networking_C|SetDebug%20network%20settings (Variables|Default|GetNetworking) (Variables|MagazineSettings|GetDebug%20mode)))

(event EventStoredinUtilityBelt
  (params (is%20stored :type Boolean))
  ;[0.494 0.3303 1] Destroy Utility belt magazines if player dies or leaves game
  (bind _output_get (Variables|Status|SetMagazine%20stored%20in%20utility%20belt is%20stored))
  (Default|UpdateActorStoredinUtilityBelt (Variables|Default|GetNetworking) _output_get (Variables|Default|GetMotionControllerPawn)))

(event EventDrop
  ;[0 0 0] Pickup/Drop
  (|DropMagazine))

(fn ConstructionScript
  (Development|SetHiddeninGame (Variables|Default|GetPickupCollision) (not (Variables|MagazineSettings|GetDebug%20mode)) false)
  (Rendering|Components|TextRender|SetText (Variables|Default|Getammo%20count) (Utilities|Text|ToText(Integer) (Variables|MagazineSettings|GetRounds)))
  (CallFunction|CreateCartridgeMeshArray)
  ;[0 0 0] replace all bullet mesh components with instanced static meshes to reduce draw calls
  (for (_array_element _array_index) (Variables|Components|GetCartridge%20meshes)
    (if (> _array_index (Variables|MagazineSettings|GetRounds))
      _
      (else
        (Components|InstancedStaticMesh|AddInstance (Variables|Default|GetISM%20cartridge) (Math|Transform|MakeTransform (Variables|/Script/Engine.SceneComponent|GetRelativeLocation _array_element) (Variables|/Script/Engine.SceneComponent|GetRelativeRotation _array_element) "1,1,1"))))
    (Components|DestroyComponent _array_element)))

(fn RemoveRound
  (Variables|MagazineSettings|SetRounds (- (Variables|MagazineSettings|GetRounds) 1))
  (if (<= (Variables|MagazineSettings|GetRounds) (Components|InstancedStaticMesh|GetInstanceCount (Variables|Default|GetISM%20cartridge)))
    (Class|InstancedStaticMeshComponent|RemoveInstance (Variables|Default|GetISM%20cartridge) (Variables|MagazineSettings|GetRounds))
    (CallFunction|MulticastRemoveCartridgeMeshInstance)))

(fn OnRepRounds
  (Rendering|Components|TextRender|SetText (Variables|Default|Getammo%20count) (Utilities|Text|ToText(Integer) (Variables|MagazineSettings|GetRounds))))

(fn AttachMagazinetoMotionControllerHand
  (Physics|SetSimulatePhysics (Variables|Default|GetMagazine) false)
  (bind _returnvalue (Transformation|AttachComponentToComponent (Variables|Default|GetMagazine) (Variables|Default|GetHand%20Mesh) (CallFunction|GetMagazineSocket) "SnapToTarget" "SnapToTarget" "SnapToTarget" false))
  (Variables|Status|SetMagazine%20ready%20to%20load (not _returnvalue)) ; Stop it instantly re-attaching when removed from gun
  (Variables|Status|SetMag%20picked%20up _returnvalue)
  (CallFunction|StopAmmoCountTextMirroringinLeftHand)
  (return _returnvalue))

(fn AttachMagazinetoGun
  (bind _returnvalue (Transformation|AttachComponentToComponent (Variables|Default|GetMagazine) (Variables|Default|GetGun%20mesh) "Magazine" "SnapToTarget" "SnapToTarget" "SnapToTarget" true)) ; attach to gun
  (CallFunction|StopAmmoCountTextMirroringinLeftHand)
  (return _returnvalue))

(fn SetInsertVariables
  (params (Gun%20mesh :type Static%20Mesh%20Component%20Object%20Reference) (Weapon :type BP%20Gun%20Object%20Reference))
  (Variables|Default|SetGun%20mesh Gun%20mesh)
  (Variables|Components|SetWeaponBP Weapon)
  (Variables|/Game/VR_Weapons/Global/Blueprints/BP_Gun.BP_Gun_C|SetMagazine (Variables|Components|GetWeaponBP) self))

(fn StopAmmoCountTextMirroringinLeftHand
  (bind _ammo_count (Variables|Default|Getammo%20count))
  (Transformation|SetWorldScale3D _ammo_count (Math|Vector|VectorGetAbs (Transformation|GetWorldScale _ammo_count))))

(fn CreateCartridgeMeshArray
  (for _array_element (Components|GetChildrenComponents (Variables|Default|GetCartridges) false) ; Go through the list of cartridge meshes
    (bind _asstatic_mesh_component (Utilities|Casting|CastToStaticMeshComponent _array_element))
    (Utilities|Array|SetArrayElem (Variables|Components|GetCartridge%20meshes) (- (Math|Conversions|ToInteger(Byte) (Utilities|String|SelectString (Utilities|String|Right (Utilities|GetObjectName _asstatic_mesh_component) 2) (Utilities|String|Right (Utilities|GetObjectName _asstatic_mesh_component) 1) (Class|KismetStringLibrary|IsNumeric (Utilities|String|Right (Utilities|GetObjectName _asstatic_mesh_component) 2)))) 1) _asstatic_mesh_component true)))

(fn InsertMagSoundEffect
  (Audio|PlaySoundatLocation (Variables|Sound|GetMagazine%20in%20audio) (Transformation|GetWorldLocation (Variables|Default|GetMagazine)) "0, 0, 0" 1.0 1.0 0.0 "/Game/VR_Weapons/Global/Audio/Small_object_Attenuation.Small_object_Attenuation" 0 0))

(fn CheckOwner
  (params (Overlapping%20actor :type Actor%20Object%20Reference))
  (bind _returnvalue (Components|GetOwner))
  (return (or (== (Components|GetOwner Overlapping%20actor) _returnvalue) (== _returnvalue 0))))

(fn GetMagazineSocket
  (return (Utilities|Select :Index (Variables|MagazineSettings|GetMagazineType) :NewEnumerator0 "None" :NewEnumerator2 "None" :NewEnumerator4 "Handgun_MagazineGripSocket" :NewEnumerator1 "Sub-machine_gun_MagazineGripSocket" :NewEnumerator5 "Assault_rifle_MagazineGripSocket" :NewEnumerator3 "Sniper_rifle_MagazineGripSocket" :NewEnumerator6 "None")))

(fn AttachtoIKMesh
  (bind _motioncontrollerpawn (Variables|Default|GetMotionControllerPawn))
  (if (Variables|/Game/VR_Weapons/Pawn/Blueprints/MotionControllerPawn.MotionControllerPawn_C|GetIK _motioncontrollerpawn)
    (Transformation|AttachComponentToComponent (VehicleSound|GetRootComponent) (Variables|/Script/Engine.Character|GetMesh _motioncontrollerpawn) (select (Utilities|Enum|Equal(Enum) (Variables|MotionController|GetHand) "Right") "hand_r" "hand_l") "KeepWorld" "KeepWorld" "KeepWorld" false)
    (Transformation|SetRelativeTransform (Variables|Default|GetMagazine) (Transformation|GetSocketTransform (Variables|Default|GetHand%20Mesh) (CallFunction|GetMagazineSocket) "RTS_ParentBoneSpace") false false)))

(fn ClearVariables
  (Variables|Status|SetMag%20picked%20up false)
  (Variables|MotionController|SetMotionController 0) ; remove old motion controller reference
  (Variables|Components|SetWeaponBP 0) ; remove old gun reference
)

(fn MagRemovedSoundEffect
  (Audio|PlaySoundatLocation (Variables|Sound|GetMagazine%20out%20audio) (Transformation|GetWorldLocation (Variables|Default|GetMagazine)) "0, 0, 0" 1.0 1.0 0.0 "/Game/VR_Weapons/Global/Audio/Small_object_Attenuation.Small_object_Attenuation" 0 0) ; click sound effect
)

(fn OnRepForceAttachonSpawn
  (Transformation|SetWorldScale3D (Variables|Default|GetMagazine) "1.000000,1.000000,1.000000")
  (CallFunction|AttachMagazinetoGun))

(fn MagInsertConditions
  (params (Weapon :type BP%20Gun%20Object%20Reference))
  (return (Math|Boolean|ANDBoolean (not (Variables|/Game/VR_Weapons/Global/Blueprints/BP_Gun.BP_Gun_C|GetWeapon%20stored%20in%20utility%20belt Weapon)) (not (Class|SceneComponent|IsAnySimulatingPhysics (Variables|/Game/VR_Weapons/Global/Blueprints/BP_Gun.BP_Gun_C|GetGun%20mesh Weapon))) (Variables|/Game/VR_Weapons/Global/Blueprints/BP_Gun.BP_Gun_C|GetLocally%20controlled Weapon))))

(fn OnRepTest
  (if (Variables|Status|GetMagazine%20attached)
    (bind _attach_successful (CallFunction|AttachMagazinetoGun))
    (if (not _attach_successful)
      (CallFunction|AttachFailed))))

(event Custom|Server%20mag%20release
  ;[0.494 0.3303 1] Replicate on server
  (Variables|Status|SetMagazine%20ready%20to%20load false)
  (Variables|Status|SetLocally%20controlled false)
  (Variables|/Game/VR_Weapons/Global/Blueprints/BP_Gun.BP_Gun_C|SetMagazine (Variables|Components|GetWeaponBP) 0) ; remove mag reference in BP_gun\nso new magazines can be inserted
  (Collision|SetCollisionResponsetoChannel (Variables|Default|GetMagazine) "ECC_GameTraceChannel4" "ECR_Ignore") ; temporarily turn off collisions to allow \nmag to fall out smoothly
  (Utilities|FlowControl|Delay 0.75) ; delay to stop mag instantly re-attaching \nor getting stuck in gun collision
  (Collision|SetCollisionResponsetoChannel (Variables|Default|GetMagazine) "ECC_GameTraceChannel4" "ECR_Block") ; reset collision so the magazine can collide and be re-attached
  (Variables|Status|SetMagazine%20ready%20to%20load true) ; magazine is now ready to be loaded into a gun
  (if (not (Variables|Status|GetMag%20picked%20up)) ; Check mag has not been picked up \nbefore removing owner and weapon ref
    (Variables|Components|SetWeaponBP 0)
    (Actor|SetOwner 0) ; remove network owner
    (return)))

(event Custom|Multicast%20mag%20remove%20from%20gun%20sound%20fx
  ;[0.494 0.3303 1] Play sound effect on all clients
  (if (not (Variables|Status|GetLocally%20controlled))
    (CallFunction|MagRemovedSoundEffect)))

(event Custom|Server%20attach
  (params (Hand%20Mesh :type Scene%20Component%20Object%20Reference) (MotionController :type BP%20Motion%20Controller%20Object%20Reference) (MotionControllerPawn :type Motion%20Controller%20Pawn%20Object%20Reference) (Hand :type EControllerHand%20Enum :default "Left"))
  (bind _networking (Variables|Default|GetNetworking))
  (bind _debug_mode (Variables|MagazineSettings|GetDebug%20mode))
  ;[0.494 0.3303 1] Server set variables
  (Variables|Default|SetHand%20Mesh Hand%20Mesh)
  (Variables|MotionController|SetMotionController MotionController)
  (Variables|Default|SetMotionControllerPawn MotionControllerPawn)
  (Variables|MotionController|SetHand Hand)
  (Variables|Status|SetMagazine%20stored%20in%20utility%20belt false)
  ;[0.494 0.3303 1] Server attach mag
  (bind _attached (CallFunction|AttachMagazinetoMotionControllerHand))
  (Utilities|FlowControl|Sequence
    (:then_0
      (if _attached
        (Development|PrintString "Mag picked up" _debug_mode _debug_mode "(R=0.032452,G=1.000000,B=0.000000,A=1.000000)")
        (CallFunction|StoredinUtilityBelt false) ; mag is only destroyed when player \nleaves if stored in utility belt
        ;[0.494 0.3303 1] Simulate physics on this actor
        ; if player quits the session unexpectedly
        (Default|DropActorifPlayerLeavesGame _networking) ; make networking component checks owning player is still in the session
        (EventDispatchers|BindEventtoSimulatePhysicsonPlayerQuit _networking (delegate Custom|Player%20quit%20session)) ; bind to event so mag doesn't remain floating if player leaves without dropping
        (Utilities|IsValid (Variables|Components|GetWeaponBP) ; is this mag being removed from a gun
          (:Is%20Valid
            (Variables|/Game/VR_Weapons/Global/Blueprints/BP_Gun.BP_Gun_C|SetMagazine (Variables|Components|GetWeaponBP) 0) ; when magazine is picked up it is no longer attached to the gun, \ntherefore destroy magazine reference in WeaponBP to disable firing
            ;[0.494 0.3303 1] Play sound effect on all clients
            (CallFunction|MulticastMagRemovefromGunSoundFx)
            (Variables|Components|SetWeaponBP 0) ; remove weapon ref for this magazine \nas it can no longer be attached to the weapon
          ))
        (else
          (Development|PrintString "Mag not picked up" _debug_mode _debug_mode "(R=1.000000,G=0.046875,B=0.046875,A=1.000000)"))))
    (:then_1
      (Utilities|FlowControl|Delay 0.25)
      (Variables|Status|SetMagazine%20ready%20to%20load true) ; allow the user to grab the mag \nwithout it instantly re-attaching\nto the gun's mag well
    )))

(event Custom|Player%20quit%20session
  ;[0.494 0.3303 1] Simulate physics on this actor
  ; if player quits the session unexpectedly
  (Physics|SetSimulatePhysics (Variables|Default|GetMagazine) true))

(event Custom|Server%20drop
  (params (Impulse :type Vector))
  ;[0.494 0.3303 1] Drop and update variables on server
  ;[0 0 0] Drop magazine actor
  (Default|ReplicateActorThrowing (Variables|Default|GetNetworking) (Variables|Default|GetMagazine) Impulse)
  (Variables|Status|SetMagazine%20attached false)
  (CallFunction|ClearVariables)
  (Actor|SetOwner 0)
  ;[0.494 0.3303 1] This actor has been dropped so should no longer
  ; be affected by the player leaving the game or dying
  (Default|ActorDropped (Variables|Default|GetNetworking) (Variables|Default|GetMotionControllerPawn))
  (|Spawnnew(autospawn)magazineifempty)
  (return))

(event Custom|Server%20insert%20magazine
  (params (Gun%20mesh :type Static%20Mesh%20Component%20Object%20Reference) (Weapon :type BP%20Gun%20Object%20Reference))
  (bind _networking (Variables|Default|GetNetworking))
  ;[0.494 0.3303 1] Update on server
  (CallFunction|SetInsertVariables Gun%20mesh Weapon)
  (Variables|Status|SetMagazine%20attached true)
  (Variables|Status|SetMagazine%20ready%20to%20load false)
  (Utilities|FlowControl|Sequence
    (:then_0
      ;[0.494 0.3303 1] Play sound effect on all clients
      (CallFunction|MulticastSoundEffect))
    (:then_1
      ;[0.494 0.3303 1] Mag is not actually dropped but update networking
      ; component as if it is, now that it's attached to a gun
      (if (Variables|Status|GetMag%20picked%20up)
        (Default|ActorDropped _networking (Variables|Default|GetMotionControllerPawn))
        (else
          (Default|ActorDropped _networking))))))

(event Custom|Multicast%20sound%20effect
  ;[0.494 0.3303 1] Play sound effect on all clients
  (if (not (Variables|Status|GetLocally%20controlled))
    (CallFunction|InsertMagSoundEffect)))

(event Custom|Force%20insert%20on%20spawn
  (params (Gun :type BP%20Gun%20Object%20Reference))
  ;[0 0 0] Attach on spawn (Utility belt)
  (CallFunction|SetInsertVariables (Variables|/Game/VR_Weapons/Global/Blueprints/BP_Gun.BP_Gun_C|GetGun%20mesh Gun) Gun)
  (Variables|Status|SetMagazine%20ready%20to%20load false)
  (Variables|Default|SetForce%20attach%20on%20spawn true))

(event Custom|Attach%20failed
  ;[0.494 0.3303 1] Resolve attach failed (sometimes happens for new players joining session)
  (bind _attach_successful (CallFunction|AttachMagazinetoGun))
  (if (not _attach_successful) ; keep looping until attach is successful
    (Utilities|FlowControl|Delay 0.1) ; delay between loops
    (Utilities|FlowControl|DoN 30 ; limit loops
      (:Exit
        (CallFunction|AttachFailed)))))

(fn GripHandGuard
  (params (Hand :type BP%20Motion%20Controller%20Object%20Reference))
  (return false 0 "NewEnumerator0"))

(fn InsertMagazine
  (params (OverlappedComponent :type Primitive%20Component%20Object%20Reference) (WeaponType :type E_WeaponType%20Enum :default "NewEnumerator0"))
  (return false 0 0))

(fn Pickup
  (params (Hand :type EControllerHand%20Enum :default "Left") (Grip%20or%20grab :type E_GrabType%20Enum :default "NewEnumerator1") (Motion%20Controller%20Actor :type BP%20Motion%20Controller%20Object%20Reference) (AttachTo :type Scene%20Component%20Object%20Reference))
  (CallFunction|PickupEvent Grip%20or%20grab Motion%20Controller%20Actor Hand AttachTo)
  (return (Variables|MagazineSettings|GetMagazineType) false))

(fn PullTrigger
  (return))

(fn ReleaseHandGuard
  (params (Hand :type BP%20Motion%20Controller%20Object%20Reference))
  (return))