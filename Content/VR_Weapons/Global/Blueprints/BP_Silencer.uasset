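; BP_Silencer is a networked VR pickup suppressor that players grab by hand and snap onto a compatible BP_Gun.
; Overlapping the gun's tagged collision attaches it after weapon type, ownership, re-attach cooldown and not-firing checks, with sound and haptics.
; Pickup and attachment happen locally first to hide latency, then go to the server once network ownership is set.
; Retry loops cover late ownership and failed OnRep attaches; drops replicate throw velocity.
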(event OnComponentBeginOverlap(Collision)
  (params (OverlappedComponent :type Primitive%20Component%20Object%20Reference) (OtherActor :type Actor%20Object%20Reference) (OtherComp :type Primitive%20Component%20Object%20Reference) (OtherBodyIndex :type Integer) (bFromSweep :type Boolean) (SweepResult :type Hit%20Result%20Structure%20%28by%20ref%29))
  (bind _bp_motioncontroller (Variables|Default|GetBP_MotionController))
  ;[0 0 0] Attach to gun
  (Utilities|FlowControl|Delay 0.1)
  (bind _asbp_gun (Utilities|Casting|CastToBP_Gun OtherActor))
  (if (CallFunction|GunAttachConditions OtherComp _asbp_gun)
    (Utilities|IsGunFiring (Variables|/Game/VR_Weapons/Global/Blueprints/BP_Gun.BP_Gun_C|GetAutomatic%20shots%20sound _asbp_gun)
      (:Not%20firing
        (Variables|Default|SetBP_gun _asbp_gun) ; create bp gun reference
        (CallFunction|AttachSilencertoGun)
        ;;[0.1302 0.1302 0.1302] FX
        (Audio|PlaySoundatLocation "/Game/VR_Weapons/Global/Audio/Silencer_attach_Cue.Silencer_attach_Cue" (Transformation|GetWorldLocation (Variables|Default|GetCollision)) "0, 0, 0" 1.0 1.0 0.0 "/Game/VR_Weapons/Global/Audio/Small_object_Attenuation.Small_object_Attenuation" 0 0)
        (Utilities|IsValid _bp_motioncontroller
          (:Is%20Valid
            (Default|RumbleController _bp_motioncontroller "/Game/VR_Weapons/Pawn/Haptics/Haptics_single.Haptics_single" 0.6 false))
          (:Is%20Not%20Valid
            _))
        (Default|PlayHaptics (Variables|Default|GetBP_gun) 0.6 0.6 "/Game/VR_Weapons/Pawn/Haptics/Haptics_single.Haptics_single" false)
        (CallFunction|MotionControllerGrips)
        ;[0.494 0.3303 1] Set network owner
        (bind _asmotion_controller_pawn (Utilities|Casting|CastToMotionControllerPawn (Components|GetOwner (Variables|Default|GetBP_gun)) :!label _label)
          (:then
            (Default|ServerSetActorOwnerinPawn _asmotion_controller_pawn self)
            (Utilities|WaitforNetworkOwnertobeSet)
            ;[0.494 0.3303 1] Update on server
            (CallFunction|ServerAttachSilencer (Variables|Default|GetBP_gun)))
          (:CastFailed
            (Development|PrintString "CAST TO MOTION CONTROLLER PAWN FAILED" true true "(R=0.265625,G=0.005475,B=0.010760,A=1.000000)" 7.0)
            (Utilities|FlowControl|Delay 0.1) ; Weapon owner might not be set yet if silencer \nwas attached right after gun was picked up
            (Utilities|FlowControl|DoN 100
              (:Exit
                (goto _label)))))))))

(event Custom|Silencer%20ready%20event
  ;[0 0 0] Prevent instant re-attach
  (Variables|Default|SetSilencer%20ready false)
  (Utilities|FlowControl|Delay 0.5)
  (Variables|Default|SetSilencer%20ready true))

(event Custom|Player%20quit%20session
  ;[0.494 0.3303 1] Drop this actor if player quits session unexpectedly
  (Physics|SetSimulatePhysics (Variables|Default|GetSilencer) true))

(event Custom|Server%20attach%20silencer
  (params (BP_gun :type BP%20Gun%20Object%20Reference))
  ;[0.494 0.3303 1] Update on server
  ;[0.494 0.3303 1] Attach
  (Variables|Default|SetBP_gun BP_gun) ; create bp gun reference
  (Variables|Default|SetSilencer%20attached true)
  ;[0.494 0.3303 1] Update BP_gun
  (Default|AttachSilencer (Variables|Default|GetBP_gun) true self)
  ;[0.494 0.3303 1] Set owner
  (Actor|SetOwner (Components|GetOwner (Variables|Default|GetBP_gun)))
  (CallFunction|MotionControllerGrips)
  ;[0.494 0.3303 1] Sound
  (CallFunction|MulticastPlaySoundFx))

(event Custom|Server%20drop
  (params (Impulse :type Vector))
  ;[0 0 0] Drop
  ;;[0.494 0.3303 1] Drop on server
  (Default|ReplicateActorThrowing (Variables|Default|GetNetworking) (Variables|Default|GetSilencer) Impulse)
  (Variables|Default|SetSilencer%20attached false)
  (Variables|/Game/VR_Weapons/Pawn/Blueprints/BP_MotionController.BP_MotionController_C|SetSilencerGrabbed (Variables|Default|GetBP_MotionController) false)
  (Variables|Default|SetBP_gun 0)
  (Variables|Default|SetBP_MotionController 0)
  (Actor|SetOwner 0)
  ;[0.494 0.3303 1] This actor has been dropped so should no longer be affected by the player leaving the game or dying
  (Default|ActorDropped (Variables|Default|GetNetworking)))

(event Custom|Server%20pickup
  (params (Handmesh :type Scene%20Component%20Object%20Reference) (BP_MotionController :type BP%20Motion%20Controller%20Object%20Reference) (Hand :type EControllerHand%20Enum :default "Left"))
  (bind _networking (Variables|Default|GetNetworking))
  (bind _bp_gun (Variables|Default|GetBP_gun))
  ;[0.494 0.3303 1] Pickup on server
  (Variables|Default|SetHandmesh Handmesh)
  (bind _output_get (Variables|Default|SetBP_MotionController BP_MotionController))
  (Variables|/Game/VR_Weapons/Pawn/Blueprints/BP_MotionController.BP_MotionController_C|SetSilencerGrabbed _output_get true)
  (Variables|Default|SetHand Hand)
  (Physics|SetSimulatePhysics (Variables|Default|GetSilencer) false)
  (Utilities|IsValid _bp_gun
    (:Is%20Valid
      (Default|AttachSilencer _bp_gun false) ; update BPgun if the silencer has been removed
    )
    (:Is%20Not%20Valid
      _))
  ;[0.494 0.3303 1] Drop this actor if player quits session unexpectedly
  (Default|DropActorifPlayerLeavesGame _networking) ; Make networking component checks owning player is still in the session
  (EventDispatchers|BindEventtoSimulatePhysicsonPlayerQuit _networking (delegate Custom|Player%20quit%20session)) ; bind to event so silencer doesn't remain floating if player leaves without dropping
  (CallFunction|AttachSilencertoHand))

(event Custom|Pickup%20event
  ;[0.494 0.3303 1] Pickup
  (Utilities|WaitforNetworkOwnertobeSet)
  (Development|PrintString "Silencer pick up!")
  (CallFunction|ServerPickup (Variables|Default|GetHandmesh) (Variables|Default|GetBP_MotionController) (Variables|Default|GetHand)))

(event Custom|Multicast%20play%20sound%20fx
  ;[0.494 0.3303 1] Sound
  (if (not (Variables|/Game/VR_Weapons/Global/Blueprints/BP_Gun.BP_Gun_C|GetLocally%20controlled (Variables|Default|GetBP_gun)))
    (Audio|PlaySoundatLocation "/Game/VR_Weapons/Global/Audio/Silencer_attach_Cue.Silencer_attach_Cue" (Transformation|GetWorldLocation (Variables|Default|GetCollision)) "0, 0, 0" 1.0 1.0 0.0 "/Game/VR_Weapons/Global/Audio/Small_object_Attenuation.Small_object_Attenuation" 0 0)))

(event Custom|Attach%20failed
  ;[0.494 0.3303 1] Attach failed (sometimes happens for new players joining session)
  (bind _successfully_attached (CallFunction|AttachSilencertoGun))
  (if (not _successfully_attached) ; keep looping until attach is successful
    (Utilities|FlowControl|Delay 0.1) ; delay between loops
    (Utilities|FlowControl|DoN 30 ; limit loops
      (:Exit
        (CallFunction|AttachFailed)
        (Development|PrintString "Silencer attached failed" true true "(R=1.000000,G=0.000000,B=0.000000,A=1.000000)" 4.0)))))

(event Collision|EventActorBeginOverlap
  (params (OtherActor :type Actor%20Object%20Reference)))

(event EventTick
  (params (DeltaSeconds :type Float%20%28single-precision%29)))

(event EventDrop
  (bind _silencer (Variables|Default|GetSilencer))
  ;[0 0 0] Drop
  (Variables|/Game/VR_Weapons/Pawn/Blueprints/BP_MotionController.BP_MotionController_C|SetSilencerGrabbed (Variables|Default|GetBP_MotionController) false)
  (Physics|SetSimulatePhysics _silencer true)
  (Transformation|DetachFromActor "KeepWorld" "KeepWorld" "KeepWorld")
  ;;[0.494 0.3303 1] Drop on server
  (CallFunction|ServerDrop (Transformation|GetComponentVelocity _silencer)))

(event EventBeginPlay
  ;[0 0 0] Simulate physics on begin play
  (if (and (Variables|Default|GetStart%20Simulating%20Physics) (Ability|HasAuthority))
    (Physics|SetSimulatePhysics (Variables|Default|GetSilencer) true)))

(fn ConstructionScript)

(fn AttachSilencertoHand
  (bind _silencer (Variables|Default|GetSilencer))
  (Physics|SetSimulatePhysics _silencer false)
  (bind _returnvalue (Transformation|AttachComponentToComponent _silencer (Variables|Default|GetHandmesh) (select (Utilities|Enum|Equal(Enum) (Variables|Default|GetWeapon%20Type) "NewEnumerator4") "SilencerHandgunGripSocket" "SilencerGripSocket") "SnapToTarget" "SnapToTarget" "SnapToTarget" true))
  (return _returnvalue))

(fn CheckOwner
  (params (Owning%20actor :type Actor%20Object%20Reference))
  (bind _returnvalue (Components|GetOwner))
  (return (or (== (Components|GetOwner Owning%20actor) _returnvalue) (== _returnvalue 0))))

(fn AttachSilencertoGun
  (bind _returnvalue (Transformation|AttachComponentToComponent (Variables|Default|GetSilencer) (Variables|/Game/VR_Weapons/Global/Blueprints/BP_Gun.BP_Gun_C|GetGun%20mesh (Variables|Default|GetBP_gun)) "Silencer" "SnapToTarget" "SnapToTarget" "SnapToTarget" true)) ; attach to gun
  (return _returnvalue))

(fn MotionControllerGrips
  (bind _bp_motioncontroller (Variables|Default|GetBP_MotionController))
  ;[0.07812 0.07812 0.07812] update grips
  (Utilities|IsValid _bp_motioncontroller
    (:Is%20Valid
      (Variables|/Game/VR_Weapons/Pawn/Blueprints/BP_MotionController.BP_MotionController_C|SetSilencerGrabbed _bp_motioncontroller false))))

(fn SetNetworkOwner
  (bind _asmotion_controller_pawn (Utilities|Casting|CastToMotionControllerPawn (Components|GetOwner (Variables|Default|GetBP_MotionController))))
  (Default|ServerSetActorOwnerinPawn _asmotion_controller_pawn self))

(fn GunAttachConditions
  (params (Collision%20box :type Actor%20Component%20Object%20Reference) (BP_Gun :type BP%20Gun%20Object%20Reference))
  (return (Math|Boolean|ANDBoolean (Components|ComponentHasTag Collision%20box "Silencer") (Variables|/Game/VR_Weapons/Global/Blueprints/BP_Gun.BP_Gun_C|GetLocally%20controlled BP_Gun) (Utilities|Enum|Equal(Enum) (Variables|/Game/VR_Weapons/Global/Blueprints/BP_Gun.BP_Gun_C|GetWeapon BP_Gun) (Variables|Default|GetWeapon%20Type)) (Variables|Default|GetSilencer%20ready) (not (Variables|/Game/VR_Weapons/Global/Blueprints/BP_Gun.BP_Gun_C|GetSilencer%20attached BP_Gun)) (CallFunction|CheckOwner BP_Gun))))

(fn OnRepSilencerAttached
  (if (Variables|Default|GetSilencer%20attached)
    (bind _successfully_attached (CallFunction|AttachSilencertoGun))
    (if (not _successfully_attached)
      (CallFunction|AttachFailed))))

(fn GripHandGuard
  (params (Hand :type BP%20Motion%20Controller%20Object%20Reference))
  (return false 0 "NewEnumerator0"))

(fn InsertMagazine
  (params (OverlappedComponent :type Primitive%20Component%20Object%20Reference) (WeaponType :type E_WeaponType%20Enum :default "NewEnumerator0"))
  (return false 0 0))

(fn Pickup
  (params (Hand :type EControllerHand%20Enum :default "Left") (Grip%20or%20grab :type E_GrabType%20Enum :default "NewEnumerator1") (Motion%20Controller%20Actor :type BP%20Motion%20Controller%20Object%20Reference) (AttachTo :type Scene%20Component%20Object%20Reference))
  (switch Utilities|FlowControl|Switch|SwitchonE_GrabType Grip%20or%20grab
    (:NewEnumerator1
      (if (CallFunction|CheckOwner Motion%20Controller%20Actor)
        (Variables|Default|SetBP_MotionController Motion%20Controller%20Actor)
        (Variables|Default|SetHandmesh AttachTo)
        (Variables|Default|SetHand Hand)
        (CallFunction|SilencerReadyEvent)
        (bind _returnvalue (CallFunction|AttachSilencertoHand)) ; attach locally first to avoid network delay
        (if _returnvalue
          (Variables|/Game/VR_Weapons/Pawn/Blueprints/BP_MotionController.BP_MotionController_C|SetSilencerGrabbed (Variables|Default|GetBP_MotionController) true)
          (bind _asmotion_controller_pawn (Utilities|Casting|CastToMotionControllerPawn (Components|GetOwner (Variables|Default|GetBP_MotionController))))
          (Default|ServerSetActorOwnerinPawn _asmotion_controller_pawn self)
          (CallFunction|PickupEvent)
          (return (Variables|Default|GetWeapon%20Type) false)
          (else
            (Development|PrintString "Silencer pickup failed" true true "(R=1.000000,G=0.000000,B=0.006082,A=1.000000)")))))))

(fn PullTrigger
  (return))