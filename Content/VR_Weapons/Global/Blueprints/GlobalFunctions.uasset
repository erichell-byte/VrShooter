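; Global function library for VR weapons, providing an Oculus Quest device check and a bullet ricochet test.
; The ricochet test rejects wood and flesh surfaces, while a missing physical material skips that filter.
; It then requires a shallow impact, judged by the dot product of normal and trace direction, a minimum distance and a weighted random roll.
; An optional debug mode prints that dot value and draws the mirrored bounce direction.
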(fn IsOculusQuestDevice
  (bind _returnvalue (Class|OculusFunctionLibrary|GetDeviceType))
  (return (or (Utilities|Enum|Equal(Enum) _returnvalue "OculusQuest") (Utilities|Enum|Equal(Enum) _returnvalue "OculusQuest2"))))

(fn CalculateRicochetAngle
  (params (Max%20angle%20for%20ricochet :type Float%20%28single-precision%29) (Min%20distance%20for%20ricochet :type Float%20%28single-precision%29) (Distance :type Float%20%28single-precision%29) (Trace%20direction :type Vector) (Hit%20Location :type Vector) (Impact%20Normal :type Vector) (Likelihood%20of%20ricochet :type Float%20%28single-precision%29) (Debug%20ricochet :type Boolean) (Physical%20material :type Physical%20Material%20Object%20Reference))
  (bind _returnvalue (Math|Vector|Normalize Impact%20Normal))
  (bind _returnvalue_2 (Math|Vector|Normalize Trace%20direction))
  (bind _returnvalue_3 (Math|Vector|DotProduct _returnvalue _returnvalue_2))
  (bind _returnvalue_4 (Math|Float|Absolute(Float) _returnvalue_3))
  (if (!= Physical%20material 0)
    (if (Utilities|Select :Index (Variables|/Script/PhysicsCore.PhysicalMaterial|GetSurfaceType Physical%20material) :SurfaceType_Default true :SurfaceType1 true :SurfaceType2 false :SurfaceType3 true :SurfaceType4 false :SurfaceType5 false)
      _
      (else
        (return false))))
  (Development|PrintString 0 (Utilities|String|Append "Impact angle: " (Utilities|String|ToString(Float) _returnvalue_4)) Debug%20ricochet Debug%20ricochet "(R=0.355838,G=0.092733,B=1.000000,A=1.000000)")
  (if Debug%20ricochet
    (Rendering|Debug|DrawDebugLine 0 Hit%20Location (+ Hit%20Location (* (Math|Vector|Normalize (Math|Vector|MirrorVectorbyNormal Trace%20direction Impact%20Normal)) 2e+02)) "(R=0.000000,G=1.000000,B=0.950757,A=1.000000)" 2.0 0.5))
  (return (Math|Boolean|ANDBoolean (< _returnvalue_4 Max%20angle%20for%20ricochet) (> Distance Min%20distance%20for%20ricochet) (Math|Random|RandomBoolwithWeight Likelihood%20of%20ricochet))))